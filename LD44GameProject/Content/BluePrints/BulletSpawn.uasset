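; BulletSpawn is a spawner actor that can fire Bullet actors, though firing is not currently wired to any event.
; On BeginPlay it starts a looping one-second timer that decrements IntValue and prints it, with no lower limit or link to firing.
; FireProjectile spawns a Bullet slightly in front of the actor along its rotation, always spawning regardless of collision, but its only call in the event graph never runs.
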(event `self.ReceiveBeginPlay`
  (`KismetSystemLibrary.K2_SetTimer` null "Timer" 1.0 true))

(fn `FireProjectile`
  (bind _returnvalue (`self.K2_GetActorRotation`))
  (`|SpawnActorFromClass` "/Game/BluePrints/Bullet.Bullet_C" (`KismetMathLibrary.MakeTransform` (+ (`self.K2_GetActorLocation`) (* (`KismetMathLibrary.GetForwardVector` _returnvalue) 50.0)) _returnvalue) "AlwaysSpawn" "OverrideRootScale" null null))

(fn `Timer`
  (bind _output_get (set `self.intValue` (- (`self.intValue`) 1)))
  (`KismetSystemLibrary.PrintString` (`KismetStringLibrary.Conv_IntToString` _output_get)))

(fn `UserConstructionScript`)