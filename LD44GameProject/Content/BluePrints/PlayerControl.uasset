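; Player controller for a mouse-aimed shooter that drives the controlled pawn.
; Axis inputs move the pawn along fixed world X and Y, while Tick sets its yaw toward the deprojected mouse world location.
; Fire calls FireBullets on the Player reference cached at BeginPlay.
; Right-click runs a debug visibility trace from the pawn to the mouse location and prints the hit actor's name.
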(event `InputAxis|Forward`
  (params (AxisValue :type "Float (single-precision)"))
  ;[1 1 1] Player Movement
  (`Pawn.AddMovementInput` (`self.K2_GetPawn`) (1.0 0.0 0.0) AxisValue false))

(event `InputAxis|Lateral`
  (params (AxisValue :type "Float (single-precision)"))
  ;[1 1 1] Player Movement
  (`Pawn.AddMovementInput` (`self.K2_GetPawn`) (0.0 1.0 0.0) AxisValue false))

(event `self.ReceiveTick`
  (params (DeltaSeconds :type "Float (single-precision)"))
  (bind _returnvalue (`self.K2_GetPawn`))
  ;[1 1 1] Rotate player to point forward towards mouse cursor
  (`self.K2_SetActorRotation` _returnvalue (`KismetMathLibrary.MakeRotator` 0.0 0.0 (.yaw (`KismetMathLibrary.FindLookAtRotation` (`self.K2_GetActorLocation` _returnvalue) (`self.DeprojectMousePositionToWorld`)))) false))

(event `InputAction|Fire`
  (params (Key :type "Key Structure"))
  ;[1 1 1] Bullet fire system (player)
  (:`Pressed`
    (`/Game/BluePrints/Player.FireBullets` (`self.PlayerCharacter`))))

(event `Key|RightMouseButton`
  (params (Key :type "Key Structure"))
  ;[1 1 1] Raycast Logic
  (:`Pressed`
    (bind _outhit (`KismetSystemLibrary.LineTraceSingle` :`Start` (`self.K2_GetActorLocation` (`self.K2_GetPawn`)) :`End` (`self.DeprojectMousePositionToWorld`) :`TraceChannel` "TraceTypeQuery1" :`DrawDebugType` "ForDuration"))
    (`KismetSystemLibrary.PrintString` (`KismetSystemLibrary.GetDisplayName` (`.HitActor` (`GameplayStatics.BreakHitResult` _outhit))))))

(event `self.ReceiveBeginPlay`
  ;[1 1 1] Store reference to player
  (bind _asplayer (cast `/Game/BluePrints/Player` (`self.K2_GetPawn`))
    (:`then`
      (set `self.PlayerCharacter` _asplayer))
    (:`CastFailed`
      (`KismetSystemLibrary.PrintString` "Initial cast failed"))))

(fn `UserConstructionScript`)